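; Blueprint for the killer tree, which creates the Life HUD and gains blood and a kill count from slain NPC units.
; Each tick it looks for a node on floors 2 to 6 and orders that floor's AI list to attack it.
; Kills trigger effects, death animations, AI alerts and a one-second burst of the otherwise paused root animation.
; Kid units double as menu choices, opening the GGJ_ART level or quitting when killed.
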(event `self.ReceiveBeginPlay`
  (set `SkeletalMeshComponent.bPauseAnims` true (`|GetArrayItem` (`self.K2_GetComponentsByClass` (`self.RootSpawnPosition`) "/Script/Engine.SkeletalMeshComponent")))
  (bind _returnvalue (`|CreateWidget` "/Game/Life.Life_C" null null))
  (set `/Game/Life.Tree` self _returnvalue)
  (`UserWidget.AddToViewport` _returnvalue 0))

(event `self.ReceiveTick`
  (params (DeltaSeconds :type "Float (single-precision)"))
  (bind _returnvalue (`self.IsANodeInThisFloor` 2))
  (if (`KismetSystemLibrary.IsValid` _returnvalue)
    (for _array_element (`self.ListAI2`)
      (`/Game/Character/BP_Unit.Attaaaaaaack` _array_element (`self.K2_GetActorLocation` _returnvalue) _returnvalue)))
  (bind _returnvalue_2 (`self.IsANodeInThisFloor` 3))
  (if (`KismetSystemLibrary.IsValid` _returnvalue_2)
    (for _array_element_2 (`self.ListAI3`)
      (`/Game/Character/BP_Unit.Attaaaaaaack` _array_element_2 (`self.K2_GetActorLocation` _returnvalue_2) _returnvalue_2)
      (bind _returnvalue_3 (`self.IsANodeInThisFloor` 5 :!label _label))
      (if (`KismetSystemLibrary.IsValid` _returnvalue_3)
        (for _array_element_3 (`self.ListAi5`)
          (`/Game/Character/BP_Unit.Attaaaaaaack` _array_element_3 (`self.K2_GetActorLocation` _returnvalue_3) _returnvalue_3)
          (bind _returnvalue_4 (`self.IsANodeInThisFloor` 6 :!label _label_2))
          (if (`KismetSystemLibrary.IsValid` _returnvalue_4)
            (for _array_element_4 (`self.ListAI6`)
              (`/Game/Character/BP_Unit.Attaaaaaaack` _array_element_4 (`self.K2_GetActorLocation` _returnvalue_4) _returnvalue_4)
              (bind _returnvalue_5 (`self.IsANodeInThisFloor` 4 :!label _label_3))
              (if (`KismetSystemLibrary.IsValid` _returnvalue_5)
                (for _array_element_5 (`self.ListAI4`)
                  (`/Game/Character/BP_Unit.Attaaaaaaack` _array_element_5 (`self.K2_GetActorLocation` _returnvalue_5) _returnvalue_5))))
            (else
              (goto _label_3))))
        (else
          (goto _label_2))))
    (else
      (goto _label))))

(event `self.OnKillNPC`
  (params (Actor :type "Actor Object Reference"))
  (bind _asbp_unit (cast `/Game/Character/BP_Unit` Actor))
  (`GameplayStatics.PlaySound2D` "/Game/Sounds/slash.slash" 1.0 1.0 0.0 null null)
  (bind _niagara (`/Game/Character/BP_Unit.Niagara` _asbp_unit))
  (`NiagaraComponent.SetVariableVec3` _niagara "Impact_Direction" (0.0 0.0 0.0))
  (`ActorComponent.Activate` _niagara false)
  (bind _asbp_unit_kid (cast `/Game/Character/BP_Unit_Kid` Actor :!label _label_4)
    (:`then`
      (bind _mesh (`Character.Mesh` _asbp_unit))
      (`SkeletalMeshComponent.PlayAnimation` _mesh "/Game/Character/A_Peasant_Dead_DeathFront_1_.A_Peasant_Dead_DeathFront_1_" false)
      (if (`/Game/Character/BP_Unit_Kid.isStart` _asbp_unit_kid)
        (`KismetSystemLibrary.Delay` 0.4)
        (`GameplayStatics.OpenLevelBySoftObjectPtr` "/Game/ART/GGJ_ART.GGJ_ART")
        (else
          (`KismetSystemLibrary.Delay` 0.4)
          (`KismetSystemLibrary.QuitGame` null "Quit"))))
    (:`CastFailed`
      (`SkeletalMeshComponent.PlayAnimation` _mesh "/Game/Character/Peasant_Old/A_Peasant_Dead_DeathBack.A_Peasant_Dead_DeathBack" false)
      (if (not (`/Game/Character/BP_Unit.IsDead` _asbp_unit))
        (`GameplayStatics.PlaySound2D` "/Game/Sounds/Shout.Shout" 1.0 1.0 0.0 null null)
        (set `/Game/Character/BP_Unit.IsDead` true _asbp_unit)
        (set `self.BloodAmount` (+ (`self.BloodAmount`) (`self.BloodGain`)))
        (`/Engine/EditorBlueprintResources/StandardMacros.IncrementInt` (`self.NbKills`)
          (:`  `
            (bind _alertai (`/Game/Character/BP_Unit.AlertAI` _asbp_unit))
            (`/Engine/EditorBlueprintResources/StandardMacros.IsValid` _alertai
              (:`Is Valid`
                (`/Game/Character/BP_Unit.Alert` _alertai))
              (:`Is Not Valid`
                _))
            (set `SkeletalMeshComponent.bPauseAnims` false (`|GetArrayItem` (`self.K2_GetComponentsByClass` (`self.RootSpawnPosition`) "/Script/Engine.SkeletalMeshComponent")))
            (`KismetSystemLibrary.K2_SetTimer` null "PauseAnim" 1.0)
            (goto _label_4)))))))

(fn `PauseAnim`
  (set `SkeletalMeshComponent.bPauseAnims` true (`|GetArrayItem` (`self.K2_GetComponentsByClass` (`self.RootSpawnPosition`) "/Script/Engine.SkeletalMeshComponent"))))

(fn `UserConstructionScript`)