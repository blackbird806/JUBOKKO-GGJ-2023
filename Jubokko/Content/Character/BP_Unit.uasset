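; Peasant unit character that can attack a target node or flee in panic.
; Alert starts a panic run and tick countdown, during which Tick's Flee shifts the actor along negative Y.
; Attaaaaaaack steps the unit along Y toward the node, then lowers its Life on a call-counted cooldown, moving by direct location changes without sweep.
; Helper functions read and write AI blackboard booleans, with BoucleCheck clearing other named states except the first.
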(event `self.ReceiveBeginPlay`
  (`KismetSystemLibrary.Delay` 0.2)
  (`self.Attack`)
  (set `self.RemainingTick` 0))

(event `Attack`
  (`SkeletalMeshComponent.PlayAnimation` (`self.Mesh`) null false))

(event `self.ReceiveTick`
  (params (DeltaSeconds :type "Float (single-precision)"))
  (`self.Flee`))

(fn `Alert`
  (`self.K2_SetActorRotation` (struct :`Yaw` 270.0))
  (`SkeletalMeshComponent.PlayAnimation` (`self.Mesh`) "/Game/Character/Peasant_Old/A_Peasant_Run_Panic.A_Peasant_Run_Panic" true)
  (set `self.RemainingTick` 30))

(fn `Attaaaaaaack`
  (params (NodeLoc :type "Vector Structure") (Node :type "TreeNode Object Reference"))
  (bind (_x _y) (`KismetMathLibrary.BreakVector3f` NodeLoc))
  (bind _lastattack (`self.LastAttack`))
  (bind _life (`TreeNode.Life` Node))
  (bind (_x_2 _y_2 _z) (`KismetMathLibrary.BreakVector3f` (`self.K2_GetActorLocation`)))
  (bind (_x_3 _y_3 _z_2) (`KismetMathLibrary.BreakVector3f` (`self.K2_GetActorLocation`)))
  (bind (_x_4 _y_4) (`KismetMathLibrary.BreakVector3f` (`self.K2_GetActorLocation`)))
  (if (not (`self.IsDead`))
    (if (not (`self.isAttacking`))
      (`SkeletalMeshComponent.PlayAnimation` (`self.Mesh`) "/Game/Character/Peasant_Old/A_Peasant_Attack_Weapon.A_Peasant_Attack_Weapon" true)
      (set `self.isAttacking` true))
    (if (or (< _y_4 (- _y 100.0)) (> _y_4 (+ _y 100.0)))
      (if (< _y_4 _y)
        (`self.K2_SetActorRotation` (struct :`Yaw` 90.0))
        (`self.K2_SetActorLocation` (`KismetMathLibrary.MakeVector` _x_2 (- _y_2 -10.0) _z))
        (else
          (`self.K2_SetActorRotation` (struct :`Yaw` 270.0))
          (`self.K2_SetActorLocation` (`KismetMathLibrary.MakeVector` _x_3 (- _y_3 10.0) _z_2))))
      (elif (> _lastattack 0)
        (`/Engine/EditorBlueprintResources/StandardMacros.DecrementInt` _lastattack)
        (else
          (set `self.LastAttack` 60)
          (`/Engine/EditorBlueprintResources/StandardMacros.DecrementInt` _life
            (:`  `
              (if (<= _life 0)
                (`SkeletalMeshComponent.PlayAnimation` (`self.Mesh`) "/Game/Character/Peasant_Old/A_Peasant_Idle_Normal.A_Peasant_Idle_Normal" true)
                (set `self.isAttacking` false)))))))))

(fn `BoucleCheck`
  (params (name :type Name))
  (for (_array_element _array_index) (`self.NamesVariable`)
    (if (not (or (== _array_element name) (== _array_index 0)))
      (`self.SetStatus` _array_element)))
  (return))

(fn `Flee`
  (bind (_x _y _z) (`KismetMathLibrary.BreakVector3f` (`self.K2_GetActorLocation`)))
  (if (not (<= (`self.RemainingTick`) 0))
    (`self.K2_SetActorLocation` (`KismetMathLibrary.MakeVector` _x (- _y 20.0) _z))
    (set `self.RemainingTick` (- (`self.RemainingTick`) 1))))

(fn `getBool`
  (params (KeyName :type "Name (by ref)"))
  (returns (ReturnValue :type Boolean))
  (return (`BlackboardComponent.GetValueAsBool` (`AIBlueprintHelperLibrary.GetBlackboard` (`AIBlueprintHelperLibrary.GetAIController` self)) KeyName)))

(fn `IsAcceleration`
  (returns (ReturnValue :type Boolean))
  (return (> (`KismetMathLibrary.VSize` (`CharacterMovementComponent.GetCurrentAcceleration` (`self.CharacterMovement`))) 0.0)))

(fn `SetStatus`
  (params (KeyName :type "Name (by ref)") (BoolValue :type Boolean))
  (`BlackboardComponent.SetValueAsBool` (`AIBlueprintHelperLibrary.GetBlackboard` (`AIBlueprintHelperLibrary.GetAIController` self)) KeyName BoolValue))

(fn `UserConstructionScript`)