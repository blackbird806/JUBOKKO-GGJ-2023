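; Peasant unit character that starts in a looping seated idle and reacts to seeing a dead PNG.
; When PawnSensing spots a pawn, it prints a debug message, then, if the peasant is alive, checks whether that pawn is a dead PNG.
; If so, it clears one named status and sets another chosen by IsSword, then passes that status name to BoucleCheck.
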(event `self.ReceiveBeginPlay`
  (`SkeletalMeshComponent.PlayAnimation` (`self.Mesh`) "/Game/Character/Peasant_Old/A_Peasant_Idle_Sit.A_Peasant_Idle_Sit" true))

(event `self.PawnSensing.OnSeePawn`
  (params (Pawn :type "Pawn Object Reference"))
  (bind _namesvariable (`self.NamesVariable`))
  (bind _output (`|GetArrayItem` _namesvariable 5))
  (bind _output_2 (`|GetArrayItem` _namesvariable 2))
  (`KismetSystemLibrary.PrintString` "Hello")
  (if (not (`self.IsDead`))
    (bind _aspng (cast `/Game/Blueprint/PNJ/PNG` Pawn))
    (if (`/Game/Blueprint/PNJ/PNG.IsDead` _aspng)
      (`self.SetStatus` (`|GetArrayItem` _namesvariable))
      (if (`self.IsSword`)
        (`self.SetStatus` _output true)
        (`self.BoucleCheck` _output)
        (else
          (`self.SetStatus` _output_2 true)
          (`self.BoucleCheck` _output_2))))))

(fn `UserConstructionScript`
  (`parent.UserConstructionScript`))