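; NPC Blueprint that reacts, while alive, to seeing a dead PNG character through PawnSensing.
; On that sighting it clears the first Blackboard state flag and sets one of two others, depending on the Sword variable.
; SetStatus writes bools to the AI controller's Blackboard by key names from NamesVariable.
; BoucleCheck keeps states exclusive by clearing every key except the chosen one and the first.
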(event `self.ReceiveBeginPlay`)

(event `self.PawnSensing.OnSeePawn`
  (params (Pawn :type "Pawn Object Reference"))
  (bind _namesvariable (`self.NamesVariable`))
  (bind _output (`|GetArrayItem` _namesvariable 5))
  (bind _output_2 (`|GetArrayItem` _namesvariable 2))
  (if (not (`self.IsDead`))
    (bind _aspng (cast `/Game/Blueprint/PNJ/PNG` Pawn))
    (if (`/Game/Blueprint/PNJ/PNG.IsDead` _aspng)
      (`self.SetStatus` (`|GetArrayItem` _namesvariable))
      (if (`self.Sword?`)
        (`self.SetStatus` _output true)
        (`self.BoucleCheck` _output)
        (else
          (`self.SetStatus` _output_2 true)
          (`self.BoucleCheck` _output_2))))))

(fn `BoucleCheck`
  (params (name :type Name))
  (for (_array_element _array_index) (`self.NamesVariable`)
    (if (not (or (== _array_element name) (== _array_index 0)))
      (`self.SetStatus` _array_element)))
  (return))

(fn `getBool`
  (params (KeyName :type "Name (by ref)"))
  (returns (ReturnValue :type Boolean))
  (return (`BlackboardComponent.GetValueAsBool` (`AIBlueprintHelperLibrary.GetBlackboard` (`AIBlueprintHelperLibrary.GetAIController` self)) KeyName)))

(fn `SetStatus`
  (params (KeyName :type "Name (by ref)") (BoolValue :type Boolean))
  (`BlackboardComponent.SetValueAsBool` (`AIBlueprintHelperLibrary.GetBlackboard` (`AIBlueprintHelperLibrary.GetAIController` self)) KeyName BoolValue))

(fn `UserConstructionScript`)